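; Enemy actor that damages the player on contact and awards score when shot.
; Collision box overlaps route to BulletHit, which adds score and destroys both enemy and bullet, or PlayerHit, which reduces health and shakes the camera.
; PlayerHit destroys the enemy and shows the restart display if player health equals exactly zero.
; The enemy also destroys itself whenever any overlap with its Sphere component ends.
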(event `self.Collision_Box.OnComponentBeginOverlap`
  (params (OverlappedComponent :type "PrimitiveComponent Object Reference") (OtherActor :type "Actor Object Reference") (OtherComp :type "PrimitiveComponent Object Reference") (OtherBodyIndex :type Integer) (bFromSweep :type Boolean) (SweepResult :type "HitResult Structure (by ref)"))
  (if (!= (`GameplayStatics.GetObjectClass` OtherActor) "/Game/InfiniteMatrix/Blueprints/Bullet.Bullet_C")
    (bind _asbp_player (cast `/Game/InfiniteMatrix/Blueprints/BP_Player` OtherActor))
    (`self.Player_Hit` _asbp_player)
    (else
      (bind _asbullet (cast `/Game/InfiniteMatrix/Blueprints/Bullet` OtherActor))
      (`self.Bullet_Hit` _asbullet))))

(event `self.Sphere.OnComponentEndOverlap`
  (params (OverlappedComponent :type "PrimitiveComponent Object Reference") (OtherActor :type "Actor Object Reference") (OtherComp :type "PrimitiveComponent Object Reference") (OtherBodyIndex :type Integer))
  (`self.K2_DestroyActor`))

(fn `Bullet_Hit`
  (params (Actor :type "/Game/InfiniteMatrix/Blueprints/Bullet Object Reference"))
  (bind _returnvalue (`GameplayStatics.GetActorOfClass` "/Game/InfiniteMatrix/Blueprints/BP_Player.BP_Player_C"))
  (set `/Game/InfiniteMatrix/Blueprints/BP_Player.Score` (+ (`/Game/InfiniteMatrix/Blueprints/BP_Player.Score` _returnvalue) 20) _returnvalue)
  (`self.K2_DestroyActor`)
  (`self.K2_DestroyActor` Actor))

(fn `Player_Hit`
  (params (Actor :type "/Game/InfiniteMatrix/Blueprints/BP_Player Object Reference"))
  (set `/Game/InfiniteMatrix/Blueprints/BP_Player.Health` (- (`/Game/InfiniteMatrix/Blueprints/BP_Player.Health` Actor) 20.0) Actor)
  (`GameplayStatics.PlayWorldCameraShake` "/Game/InfiniteMatrix/Blueprints/Camera_Shake.Camera_Shake_C" (`self.K2_GetActorLocation` Actor) 0.0 1000.0)
  (`self.K2_DestroyActor`)
  (if (== (`/Game/InfiniteMatrix/Blueprints/BP_Player.Health` Actor) 0.0)
    (`/Game/InfiniteMatrix/Blueprints/BP_Player.DisplayRestart` Actor)))

(fn `UserConstructionScript`)